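; BP_SideScrolling_NPC is a side-scrolling NPC character that gets knocked back and temporarily deactivated when interacted with.
; Interaction launches it upward and along the interactor's facing on X, stops its current movement, and sets a Deactivated flag registered by its AI State Tree.
; After DeactivationTime it clears the flag and resets the DoOnce gate that blocks repeat interactions meanwhile.
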(event Custom|Reset%20Deactivation
  ;[0.15 0.15 0.15 0.5] If Interacted with, enter a deactivation state - this is registered by the AI State Tree for this NPC - and get launched back
  (Utilities|FlowControl|DoOnce false) ; enters at Reset
)

(event EventInteraction
  (params (Interactor :type Actor%20Object%20Reference))
  ;[0.15 0.15 0.15 0.5] If Interacted with, enter a deactivation state - this is registered by the AI State Tree for this NPC - and get launched back
  (Utilities|FlowControl|DoOnce false
    (:Completed
      (Variables|NPC|SetDeactivated true)
      (Character|LaunchCharacter (Math|Vector|MakeVector (.x (* (Transformation|GetActorForwardVector Interactor) 5e+02)) 0.0 5e+02) true true)
      (Components|Movement|StopMovementImmediately (Variables|Character|GetCharacterMovement))
      (Utilities|FlowControl|Delay (Variables|NPC|GetDeactivationTime))
      (Variables|NPC|SetDeactivated false)
      (CallFunction|ResetDeactivation))))

(fn ConstructionScript)